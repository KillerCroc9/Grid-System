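; Hex grid generator actor that shows the mouse cursor and adds the W_Controls widget to the viewport on BeginPlay.
; Its events clear existing MyHexagon actors before generating a sized grid, find neighbors by Q/R coordinates, and push a computed hex distance to W_Controls.
; Grid logic is delegated to same-named functions; disconnected nodes retain older debug printing and Blueprint offset spawning, noted as moved to C++.
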(event `self.ReceiveBeginPlay`
  (bind _returnvalue (`GameplayStatics.GetPlayerController` 0))
  (set `PlayerController.bShowMouseCursor` true _returnvalue)
  (bind _returnvalue_2 (`|CreateWidget` "/Game/UI/W_Controls.W_Controls_C" _returnvalue))
  (`UserWidget.AddToViewport` _returnvalue_2 0))

(event `Generate Grid`
  (params (Size :type Integer))
  (bind _outactors (`GameplayStatics.GetAllActorsOfClass` "/Game/Blueprints/MyHexagon.MyHexagon_C"))
  (for _array_element _outactors
    (`self.K2_DestroyActor` _array_element))
  (`self.GenerateGrid` Size))

(event `Find Neighbors`
  (params (Q :type Integer) (R :type Integer))
  (`self.findNeighbors` Q R))

(event `Distance To Target`
  (params (AQ :type Integer) (AR :type Integer) (BQ :type Integer) (BR :type Integer))
  (bind _returnvalue (`self.distanceToTarget` AQ AR BQ BR))
  (bind _foundwidgets (`WidgetBlueprintLibrary.GetAllWidgetsOfClass` "/Game/UI/W_Controls.W_Controls_C"))
  (set `/Game/UI/W_Controls.Dis` _returnvalue (`|GetArrayItem` _foundwidgets)))

(fn `UserConstructionScript`)